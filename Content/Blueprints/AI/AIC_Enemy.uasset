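; AIC_Enemy is the enemy AI controller, running BT_Enemy with BB_Enemy for a possessed BP_Character.
; It mirrors the character's stun state and the assigned attack target into the blackboard.
; Every tick it sets the focal point toward a valid target only along world X, as in side-on movement, while the character can act.
; Otherwise the character keeps its current facing.
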(event Custom|OnStunnedStateChanged
  (params (isStunned :type Boolean))
  (AI|Components|Blackboard|SetValueasBool (Variables|Default|GetBlackboard) (Variables|Default|GetisStunnedKey) isStunned))

(event EventBeginPlay
  (Class|AIController|UseBlackboard "/Game/Blueprints/AI/BB_Enemy.BB_Enemy")
  (AI|RunBehaviorTree "/Game/Blueprints/AI/BT_Enemy.BT_Enemy"))

(event EventTick
  (params (DeltaSeconds :type Float%20%28single-precision%29))
  (CallFunction|SetFocusDirection))

(event EventPossess
  (params (PossessedPawn :type Pawn%20Object%20Reference))
  (bind _asbp_character (Utilities|Casting|CastToBP_Character PossessedPawn))
  (Variables|Default|SetActionCharacter _asbp_character)
  (EventDispatchers|BindEventtoStunStateChanged (Variables|Default|GetActionCharacter) (delegate Custom|OnStunnedStateChanged)))

(fn ConstructionScript)

(fn SetAttackTarget
  (params (AttackTarget :type BP%20Adventurer%20Object%20Reference))
  (AI|Components|Blackboard|SetValueasObject (Variables|Default|GetBlackboard) (Variables|Default|GetAttackTargetKey) AttackTarget)
  (Variables|Default|SetAttackTarget AttackTarget))

(fn SetFocusDirection
  (bind _actioncharacter (Variables|Default|GetActionCharacter))
  (Utilities|IsValid (Variables|Default|GetAttackTarget)
    (:Is%20Valid
      (if (Default|CanAct (Variables|Default|GetActionCharacter))
        (AI|SetFocalPoint (+ (Transformation|GetActorLocation (Variables|Default|GetActionCharacter)) (Math|Vector|MakeVector (.x (Math|Vector|GetForwardVector (Math|Rotator|FindLookatRotation (Transformation|GetActorLocation (Variables|Default|GetActionCharacter)) (Transformation|GetActorLocation (Variables|Default|GetAttackTarget))))) 0.0 0.0)))
        (else
          (AI|SetFocalPoint (+ (Transformation|GetActorLocation _actioncharacter) (Transformation|GetActorForwardVector _actioncharacter)) :!label _label))))
    (:Is%20Not%20Valid
      (goto _label))))