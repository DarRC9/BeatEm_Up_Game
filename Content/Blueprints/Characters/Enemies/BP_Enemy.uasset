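; BP_Enemy is an enemy character that aggros on the player's adventurer and hands combat targeting to its AI controller.
; When a BP_Adventurer begins overlapping the AggroRange component, it passes that actor to AIC_Enemy as the attack target.
; ReceiveDamage extends the parent's damage handling, disabling capsule collision when IsDead is true so dead enemies no longer block.
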(event OnComponentBeginOverlap(AggroRange)
  (params (OverlappedComponent :type Primitive%20Component%20Object%20Reference) (OtherActor :type Actor%20Object%20Reference) (OtherComp :type Primitive%20Component%20Object%20Reference) (OtherBodyIndex :type Integer) (bFromSweep :type Boolean) (SweepResult :type Hit%20Result%20Structure%20%28by%20ref%29))
  (bind _asbp_adventurer (Utilities|Casting|CastToBP_Adventurer OtherActor))
  (bind _asaic_enemy (Utilities|Casting|CastToAIC_Enemy (AI|GetAIController self)))
  (Default|SetAttackTarget _asaic_enemy _asbp_adventurer))

(event EventBeginPlay
  (|CallParentFunction) ; This node is disabled and will not be called.\nDrag off pins to build functionality.
)

(event Collision|EventActorBeginOverlap
  (params (OtherActor :type Actor%20Object%20Reference))
  (|CallParentFunction OtherActor) ; This node is disabled and will not be called.\nDrag off pins to build functionality.
)

(event EventTick
  (params (DeltaSeconds :type Float%20%28single-precision%29))
  (|CallParentFunction DeltaSeconds) ; This node is disabled and will not be called.\nDrag off pins to build functionality.
)

(fn ConstructionScript
  (|CallParentFunction))

(fn ReceiveDamage
  (params (Damage :type Float%20%28double-precision%29))
  (|CallParentFunction Damage)
  (if (Variables|Default|GetisDead)
    (Collision|SetCollisionEnabled (Variables|Default|GetCapsuleComponent) "NoCollision")))